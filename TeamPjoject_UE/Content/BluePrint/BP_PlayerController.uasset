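; BP_PlayerController is a player controller that lets the Space bar lower the player's HP.
; On BeginPlay it caches references to BP_GameMode and to BP_PlayerStat from player state index 0.
; Each press subtracts one HP from the player stat while it is above zero, then prints the new value, which resembles a simple test of the stat.
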(event EventBeginPlay
  (Utilities|FlowControl|Sequence
    (:then_0
      (bind _asbp_game_mode (Utilities|Casting|CastToBP_GameMode (Game|GetGameMode)))
      (Variables|Default|SetAs%20BP%20Game%20Mode _asbp_game_mode))
    (:then_1
      (bind _asbp_player_stat (Utilities|Casting|CastToBP_PlayerStat (Game|GetPlayerState 0)))
      (Variables|Default|SetAs%20BP%20Player%20Stat _asbp_player_stat))))

(event Input|KeyboardEvents|SpaceBar
  (params (Key :type Key%20Structure :default "None"))
  (:Pressed
    (if (> (Variables|/Game/BluePrint/BP_PlayerStat.BP_PlayerStat_C|GetHP (Variables|Default|GetAs%20BP%20Player%20Stat)) 0)
      (bind _output_get (Variables|/Game/BluePrint/BP_PlayerStat.BP_PlayerStat_C|SetHP (Variables|Default|GetAs%20BP%20Player%20Stat) (- (Variables|/Game/BluePrint/BP_PlayerStat.BP_PlayerStat_C|GetHP (Variables|Default|GetAs%20BP%20Player%20Stat)) 1)))
      (Development|PrintText (Utilities|Text|FormatText "HP : {HP}" _output_get)))))

(fn ConstructionScript)